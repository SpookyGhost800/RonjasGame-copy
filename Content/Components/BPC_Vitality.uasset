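; BPC_Vitality is a component that tracks health and a defeated flag for its owner.
; On BeginPlay it sets current health to max health.
; RecieveHealth subtracts incoming damage and, at zero or below, sets IsDefeated to false rather than true.
; Health is not clamped, as the ClampFloat node is unused, and Tick does nothing.
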(event `self.ReceiveBeginPlay`
  ;[1 1 1] Max health matches current health on Play
  (set `self.CurrentHealth` (`self.MaxHealth`)))

(fn `RecieveHealth`
  (params (Damage :type "Float (double-precision)"))
  (set `self.CurrentHealth` (- (`self.CurrentHealth`) Damage))
  (if (<= (`self.CurrentHealth`) 0.0)
    (set `self.IsDefeated` false)))