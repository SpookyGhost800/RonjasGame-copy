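; BP_Projectile_BASE is the base projectile Blueprint, with overlap logic that currently suits player shots against enemies.
; A sphere hit spawns the BP_VFX_ShotHit effect at the projectile's location and destroys the projectile.
; A sphere overlap with a BP_Enemy_BASE destroys that enemy outright, then calls ApplyDamage with no target set, plays the effect and destroys itself.
; A cast to BP_ActionChar_BASE is left unconnected, so player characters are not handled on overlap.
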(event `self.Sphere.OnComponentHit`
  (params (HitComponent :type "PrimitiveComponent Object Reference") (OtherActor :type "Actor Object Reference") (OtherComp :type "PrimitiveComponent Object Reference") (NormalImpulse :type "Vector Structure") (Hit :type "HitResult Structure (by ref)"))
  ;[1 1 1] This will always play when we destroy the projectile
  (`self.PlayHitEffects`)
  (`self.K2_DestroyActor`))

(event `self.Sphere.OnComponentBeginOverlap`
  (params (OverlappedComponent :type "PrimitiveComponent Object Reference") (OtherActor :type "Actor Object Reference") (OtherComp :type "PrimitiveComponent Object Reference") (OtherBodyIndex :type Integer) (bFromSweep :type Boolean) (SweepResult :type "HitResult Structure (by ref)"))
  ;[1 1 1] work for player projectiles - not for lizard - could redo all of this in our children and make sure that in the case it's a player, we cast to enemy, if enemy we cast to player (actionChar)
  (bind _asbp_enemy_base (cast `/Game/Blueprints/Characters/Enemies/BP_Enemy_BASE` OtherActor))
  (`self.K2_DestroyActor` _asbp_enemy_base)
  (`GameplayStatics.ApplyDamage` null (`self.ProjectileDamage`))
  (`self.PlayHitEffects`)
  (`self.K2_DestroyActor`))

(fn `PlayHitEffects`
  (`|SpawnActorFromClass` "/Game/Blueprints/VFX/BP_VFX_ShotHit.BP_VFX_ShotHit_C" (`KismetMathLibrary.MakeTransform` (`self.K2_GetActorLocation`) (`self.K2_GetActorRotation`)) "Undefined" "MultiplyWithRoot" null null))

(fn `UserConstructionScript`)