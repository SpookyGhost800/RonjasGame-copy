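; Base Blueprint for player projectiles that removes them once they leave the screen horizontally.
; Each Tick runs the parent logic, then projects the actor's location to screen space and compares X against the left and right viewport edges.
; Off-screen projectiles are destroyed, with PlayHitEffects called after DestroyActor.
; BeginPlay and overlap are empty, and construction defers to the parent.
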(event `self.ReceiveBeginPlay`)

(event `self.ReceiveTick`
  (params (DeltaSeconds :type "Float (single-precision)"))
  (bind _returnvalue_x (`KismetMathLibrary.BreakVector2D` (`WidgetLayoutLibrary.GetViewportSize`)))
  (bind _screenlocation (`PlayerController.ProjectWorldLocationToScreen` (`GameplayStatics.GetPlayerController` 0) (`self.K2_GetActorLocation`) false))
  ;[1 1 1] Ensure for no bugs
  (`parent.ReceiveTick` 0.0)
  ;[1 1 1] If projectile out of viewport - delete
  (if (or (>= (`KismetMathLibrary.BreakVector2D` _screenlocation) _returnvalue_x) (<= (`KismetMathLibrary.BreakVector2D` _screenlocation) 0.0))
    (`self.K2_DestroyActor`)
    (`self.PlayHitEffects`)))

(fn `UserConstructionScript`
  (`parent.UserConstructionScript`))